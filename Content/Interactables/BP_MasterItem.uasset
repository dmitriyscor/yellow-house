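; BP_MasterItem is an interactable item, likely a base class, that shows an interact prompt when the third-person character is near.
; Sphere overlap creates the WB_UI_Interact widget in a widget component, plays its PopUp animation forward on entry, and reverses it before hiding on exit.
; The CanReceiveTrace? event can also toggle the prompt animation.
; HintVisible guards against replays, and CanPressE tracks whether interaction input is allowed.
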(event `self.Sphere.OnComponentBeginOverlap`
  (params (OverlappedComponent :type "PrimitiveComponent Object Reference") (OtherActor :type "Actor Object Reference") (OtherComp :type "PrimitiveComponent Object Reference") (OtherBodyIndex :type Integer) (bFromSweep :type Boolean) (SweepResult :type "HitResult Structure (by ref)"))
  (bind _widget (`self.Widget`))
  (cast `/Game/ThirdPerson/Blueprints/BP_ThirdPersonCharacter` OtherActor)
  (if (`self.Can Interact`)
    (bind _returnvalue (`|CreateWidget` "/Game/FirstPerson/WB_UI_Interact.WB_UI_Interact_C"))
    (bind _output_get (set `self.Interaction Widget` _returnvalue))
    (`WidgetComponent.SetWidget` _widget _output_get)
    (`SceneComponent.SetVisibility` _widget true false)
    (bind _interaction_widget (`self.Interaction Widget`)
      (:`then`
        (if (not (`self.Hint Visible`))
          (`UserWidget.PlayAnimation` _interaction_widget (`/Game/FirstPerson/WB_UI_Interact.PopUp` _interaction_widget) 0.0 1 "Forward" 1.5 false)
          (set `self.Hint Visible` true)
          (set `self.Can Press E` true)))
      (:`else`))))

(event `self.Sphere.OnComponentEndOverlap`
  (params (OverlappedComponent :type "PrimitiveComponent Object Reference") (OtherActor :type "Actor Object Reference") (OtherComp :type "PrimitiveComponent Object Reference") (OtherBodyIndex :type Integer))
  (cast `/Game/ThirdPerson/Blueprints/BP_ThirdPersonCharacter` OtherActor)
  (if (`self.Can Interact`)
    (bind _interaction_widget (`self.Interaction Widget`)
      (:`then`
        (if (`self.Hint Visible`)
          (`UserWidget.PlayAnimation` _interaction_widget (`/Game/FirstPerson/WB_UI_Interact.PopUp` _interaction_widget) 0.0 1 "Reverse" 1.5 false)
          (set `self.Hint Visible` false)
          (set `self.Can Press E` false)
          (`KismetSystemLibrary.Delay` 0.15 :!label _label)
          (`Widget.RemoveFromParent` (`self.Interaction Widget`))
          (`SceneComponent.SetVisibility` (`self.Widget`) false false)))
      (:`else`))
    (else
      (goto _label))))

(event `/Game/ThirdPerson/Blueprints/BPI_Interaction.Can Receive Trace?`
  (params (`Can Interact?` :type Boolean))
  (if (`self.Can Interact`)
    (if `Can Interact?`
      (bind _interaction_widget (`self.Interaction Widget`)
        (:`then`
          (if (not (`self.Hint Visible`))
            (`UserWidget.PlayAnimation` _interaction_widget (`/Game/FirstPerson/WB_UI_Interact.PopUp` _interaction_widget) 0.0 1 "Forward" 1.5 false)
            (set `self.Hint Visible` true)
            (set `self.Can Press E` true)))
        (:`else`))
      (else
        (bind _interaction_widget_2 (`self.Interaction Widget`)
          (:`then`
            (if (`self.Hint Visible`)
              (`UserWidget.PlayAnimation` _interaction_widget_2 (`/Game/FirstPerson/WB_UI_Interact.PopUp` _interaction_widget_2) 0.0 1 "Reverse" 1.5 false)
              (set `self.Hint Visible` false)
              (set `self.Can Press E` false)))
          (:`else`))))))

(fn `UserConstructionScript`)