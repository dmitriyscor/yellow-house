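; Enemy monster character that roams, hides in shadows and hunts the player, with debug prints throughout.
; PawnSensing flags sightings and loud noises, and a random action picker chooses between idle and attack behaviors.
; Shadow hiding teleports it between random BP_Shadow actors before it exits.
; Attacks follow the player, then move to the last known location and start timer-sampled pursuit; stalking, closet actions and kill animations are stubs.
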(event `self.ReceiveBeginPlay`
  (`KismetSystemLibrary.Delay` 0.3)
  (bind _outactors (`GameplayStatics.GetAllActorsOfClass` "/Game/ThirdPerson/Blueprints/BP_ThirdPersonCharacter.BP_ThirdPersonCharacter_C"))
  (set `self.Player` (`|GetArrayItem` _outactors))
  (`self.Next Action?`))

(event `self.ReceiveTick`
  (params (DeltaSeconds :type "Float (single-precision)"))
  (`KismetSystemLibrary.PrintString` (`KismetStringLibrary.Concat_StrStr` "Player in sight: " (`KismetStringLibrary.Conv_BoolToString` (`self.Player In Sight?`)) " \nInside a Shadow:" (`KismetStringLibrary.Conv_BoolToString` (`self.Inside a Shadow?`)) " \nAttacking the Player:" (`KismetStringLibrary.Conv_BoolToString` (`self.Attacking Player?`))) true true (struct :`R` 1.0 :`G` 0.954361 :`B` 0.934119 :`A` 1.0) DeltaSeconds))

(event `Next Action?`
  ;[1 1 1] Next Action?
  (if (`self.Player In Sight?`)
    (if (not (or (`self.Attacking Player?`) (`self.Stalking Player?`)))
      (switch `int` (`KismetMathLibrary.RandomIntegerInRange` 0 1)
        (:`0`
          (`self.Stalk Player`))
        (:`1`
          (`self.Attack Player`))))
    (elif (not (`self.Player Hiding for too long?`))
      (switch `int` (`KismetMathLibrary.RandomIntegerInRange` 0 2)
        (:`0`
          (`self.Random Roam`))
        (:`1`
          (`self.Enter Nearest Shadow`))
        (:`2`
          (`self.Open Closest Closet`)))
      (else
        (`self.Teleport Inside Closet`)))))

(event `Enter the Shadow`
  ;[1 1 1] Shadow Events
  (`|AIMoveTo` self (`self.Closest Shadow Location`) null
    (:`OnSuccess`
      (set `self.Inside a Shadow?` true)
      (`SceneComponent.SetVisibility` (`self.PointLight`) true false)
      (`GameplayStatics.PlaySound2D` "/Engine/VREditor/Sounds/UI/Dockable_Window_Open.Dockable_Window_Open" 1.0 1.0 0.0 null null)
      (`self.Change Shadow`))
    (:`OnFail`
      (`self.Next Action?`))))

(event `Random Roam`
  ;[1 1 1] On Idle Actions
  (`|AIMoveTo` self (`NavigationSystemV1.K2_GetRandomReachablePointInRadius` (`SceneComponent.K2_GetComponentLocation` (`self.CapsuleComponent`)) (`KismetMathLibrary.RandomFloatInRange` 300.0 1200.0) null null) null
    (:`OnSuccess`
      _)
    (:`OnFail`
      _))
  (`KismetSystemLibrary.Delay` 3.0)
  (`self.Next Action?`))

(event `Teleport Inside Closet`
  ;[1 1 1] On Idle Actions
  ;;[1 0 0] TO DO
)

(event `Stalk Player`
  ;[1 1 1] On Player in Sight
  (if (`self.Inside a Shadow?`)
    _))

(event `Attack Player`
  ;[1 1 1] On Player in Sight
  (if (not (`self.Inside a Shadow?`))
    (`KismetArrayLibrary.Array_Clear` (`self.Player Prev Locations`))
    (if (`self.Player In Sight?`) :!label _label
      (set `self.Attacking Player?` true)
      (`|AIMoveTo` self (0.0 0.0 0.0) (`GameplayStatics.GetPlayerCharacter` 0)
        (:`then`
          (`KismetSystemLibrary.PrintString` "following")
          (`KismetSystemLibrary.Delay` 0.5)
          (set `self.Player's location` (`SceneComponent.K2_GetComponentLocation` (`Character.Mesh` (`GameplayStatics.GetPlayerCharacter` 0))))
          (goto _label))
        (:`OnSuccess`
          (set `self.Attacking Player?` false))
        (:`OnFail`
          (goto _label)))
      (else
        (set `self.Player's location` (`SceneComponent.K2_GetComponentLocation` (`Character.Mesh` (`GameplayStatics.GetPlayerCharacter` 0))))
        (set `self.Attacking Player?` false)
        (`|AIMoveTo` self (`self.Player's location`) null 10.0
          (:`OnSuccess`
            (`self.Chase` 12.0))
          (:`OnFail`
            (`self.Next Action?`)))))))

(event `Change Shadow`
  ;[1 1 1] Shadow Events
  (`GameplayStatics.PlaySound2D` "/Engine/VREditor/Sounds/UI/Dockable_Window_Drop.Dockable_Window_Drop" 1.0 1.0 0.0 null null)
  (bind _outactors (`GameplayStatics.GetAllActorsOfClass` "/Game/Enemy/BP_Shadow.BP_Shadow_C"))
  (bind _rootcomponent (`Actor.RootComponent` (`|GetArrayItem` _outactors (`KismetMathLibrary.RandomIntegerInRange` 0 (- (`KismetArrayLibrary.Array_Length` _outactors) 1)))))
  (`SceneComponent.K2_SetWorldLocationAndRotation` (`self.CapsuleComponent`) (`SceneComponent.K2_GetComponentLocation` _rootcomponent) (`SceneComponent.K2_GetComponentRotation` _rootcomponent) false true)
  (`KismetSystemLibrary.Delay` 5.0)
  (if (`self.Player In Sight?`)
    (`KismetSystemLibrary.Delay` 3.0)
    (`self.Exit the Shadow`)
    (else
      (`/Engine/EditorBlueprintResources/StandardMacros.FlipFlop`
        (:`A`
          (`self.Change Shadow`))
        (:`B`
          (`self.Exit the Shadow`))))))

(event `Enter Nearest Shadow`
  (bind _returnvalue (`KismetMathLibrary.VSize` (`self.K2_GetActorLocation`)))
  ;[1 1 1] On Idle Actions
  (bind _outactors (`GameplayStatics.GetAllActorsOfClass` "/Game/Enemy/BP_Shadow.BP_Shadow_C"))
  (for _array_element _outactors
    (bind _returnvalue_2 (`self.K2_GetActorLocation` _array_element))
    (bind _returnvalue_3 (`KismetMathLibrary.VSize` _returnvalue_2))
    (bind _returnvalue_4 (- _returnvalue _returnvalue_3))
    (`KismetSystemLibrary.PrintString` (`KismetStringLibrary.Concat_StrStr` "Monster's location:" (`KismetStringLibrary.Conv_DoubleToString` _returnvalue) " \nShadow's location:" (`KismetStringLibrary.Conv_DoubleToString` _returnvalue_3) " \nDistance (abs):" (`KismetStringLibrary.Conv_DoubleToString` _returnvalue_4)) false true (struct :`R` 1.0 :`G` 0.773286 :`A` 1.0) 20.0)
    (if (> (`KismetMathLibrary.VSize` (`self.Closest Shadow Location`)) (`KismetMathLibrary.Abs` _returnvalue_4))
      (set `self.Closest Shadow Location` _returnvalue_2)))
  (`self.Enter the Shadow`))

(event `Exit the Shadow`
  ;[1 1 1] Shadow Events
  (set `self.Inside a Shadow?` false)
  (`SceneComponent.SetVisibility` (`self.PointLight`) false false)
  (`KismetSystemLibrary.Delay` 1.0)
  (`GameplayStatics.PlaySound2D` "/Engine/VREditor/Sounds/UI/Dockable_Window_Close.Dockable_Window_Close" 1.0 1.0 0.0 null null)
  (`/Engine/EditorBlueprintResources/StandardMacros.FlipFlop`
    (:`A`
      (`self.Random Roam`))
    (:`B`
      (`self.Open Closest Closet`))))

(event `Open Closest Closet`
  ;[1 1 1] On Idle Actions
  (`self.Next Action?`))

(event `Chase`
  (params (Time :type "Float (double-precision)"))
  (`KismetSystemLibrary.PrintString` "chase sequence started")
  (bind _returnvalue (`KismetSystemLibrary.K2_SetTimerDelegate` (delegate `Check Location`) 2.0 true))
  (`KismetSystemLibrary.Delay` Time))

(event `Check Location`
  (bind _player_prev_locations (`self.Player Prev Locations`))
  (if (`KismetArrayLibrary.Array_IsValidIndex` _player_prev_locations)
    (`|AIMoveTo` self (`|GetArrayItem` _player_prev_locations) null
      (:`OnSuccess`
        (`KismetArrayLibrary.Array_Remove` _player_prev_locations))
      (:`OnFail`
        _)))
  (`KismetArrayLibrary.Array_Add` _player_prev_locations (`SceneComponent.K2_GetComponentLocation` (`Character.Mesh` (`GameplayStatics.GetPlayerCharacter` 0))))
  (`KismetSystemLibrary.PrintString` "next location"))

(event `Play Kill Animation`
  ;[1 0 0] Player Kill Anims
  (switch `int` (`KismetMathLibrary.RandomIntegerInRange` 0 3)))

(event `self.PawnSensing.OnSeePawn`
  (params (Pawn :type "Pawn Object Reference"))
  ;[1 1 1] Sensing
  ;;[1 1 1] On See Pawn
  (cast `/Game/ThirdPerson/Blueprints/BP_ThirdPersonCharacter` Pawn)
  (set `self.Player In Sight?` true)
  (`self.Next Action?`)
  (`KismetSystemLibrary.Delay` 1.0)
  (set `self.Player In Sight?` false))

(event `self.PawnSensing.OnHearNoise`
  (params (Instigator :type "Pawn Object Reference") (Location :type "Vector Structure (by ref)") (Volume :type "Float (single-precision)"))
  ;[1 1 1] Sensing
  ;;[1 0 0] On Hear Noise
  (if (> Volume 0.5)
    (`self.Investigate Noises` Location)))

(event `Investigate Noises`
  (params (Location :type "Vector Structure"))
  ;[1 1 1] Sensing
  ;;[1 0 0] On Hear Noise
  (`|AIMoveTo` self Location null 10.0))

(fn `UserConstructionScript`)