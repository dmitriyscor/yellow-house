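; Interactive in-world notebook that opens, closes and flips between two-page spreads of UMG widgets.
; A timeline rotates the cover, and animated page meshes play each turn while input is gated.
; DrawPage staggers widget swaps, with copy widgets' render targets feeding the turning pages' dynamic materials.
; Opening rebinds page-turn actions to the player's MoveLeft/MoveRight keys and adds the notebook mapping context, which closing removes.
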(event `self.ReceiveBeginPlay`
  (bind _page_righttoleft (`self.Page RightToLeft`))
  (bind _right_page_instance_material (`self.Right Page Instance Material`))
  (bind _page_lefttoright (`self.Page LeftToRight`))
  (bind _leftpageinstancematerial (`self.LeftPageInstanceMaterial`))
  (`|ExecutionSequence`
    (:`then_0`
      (bind _returnvalue (`PrimitiveComponent.CreateDynamicMaterialInstance` _page_righttoleft 0 (`PrimitiveComponent.GetMaterial` _page_righttoleft 0) "None"))
      (bind _output_get (set `self.Right Page Instance Material` _returnvalue))
      (`PrimitiveComponent.SetMaterial` (`self.Page RightToLeft`) 0 _output_get)
      (`KismetSystemLibrary.Delay` 0.1)
      (`MaterialInstanceDynamic.SetTextureParameterValue` _right_page_instance_material "WidgetRenderTarget" (`WidgetComponent.GetRenderTarget` (`self.Page A Widget Copy`)))
      (`MaterialInstanceDynamic.SetTextureParameterValue` _right_page_instance_material "WidgetRenderTarget2" (`WidgetComponent.GetRenderTarget` (`self.Page B  Widget Copy`))))
    (:`then_1`
      (bind _returnvalue_2 (`PrimitiveComponent.CreateDynamicMaterialInstance` _page_lefttoright 0 (`PrimitiveComponent.GetMaterial` _page_lefttoright 0) "None"))
      (bind _output_get_2 (set `self.LeftPageInstanceMaterial` _returnvalue_2))
      (`PrimitiveComponent.SetMaterial` (`self.Page LeftToRight`) 0 _output_get_2)
      (`KismetSystemLibrary.Delay` 0.1)
      (`MaterialInstanceDynamic.SetTextureParameterValue` _leftpageinstancematerial "WidgetRenderTarget" (`WidgetComponent.GetRenderTarget` (`self.Page A Widget Copy`)))
      (`MaterialInstanceDynamic.SetTextureParameterValue` _leftpageinstancematerial "WidgetRenderTarget2" (`WidgetComponent.GetRenderTarget` (`self.Page B  Widget Copy`))))))

(event `Open`
  (bind _imc_notebookref (`self.IMC_NotebookRef`))
  (bind _imc_notebookref_2 (`self.IMC_NotebookRef`))
  (bind _returnvalue (`EnhancedPlayerMappableKeyProfile.GetPlayerMappingRows` (`EnhancedInputUserSettings.GetCurrentKeyProfile` (`EnhancedInputSubsystemInterface.GetUserSettings` (pcsubsystem `EnhancedInputLocalPlayerSubsystem` (`GameplayStatics.GetPlayerController` 0))))))
  (set `self.Animation is Playing?` true)
  (set `self.AddMappingContext?` true)
  (`|ExecutionSequence`
    (:`then_0`
      (set `self.Book Opened?` true)
      (bind (_direction _newtrack_0) (`Timeline|Open/Close` :!label _label)
        (:`Update`
          (`SceneComponent.K2_SetRelativeRotation` (`self.SM_NotebookA`) (`KismetMathLibrary.MakeRotator` 0.0 (`KismetMathLibrary.Lerp` -179.0 0.0 _newtrack_0)) false false))
        (:`Finished`
          (set `self.Animation is Playing?` false)
          (`self.Draw Page` (`self.Current Page`))
          (if (`self.AddMappingContext?`)
            (`|ExecutionSequence`
              (:`then_0`
                (bind _result (`BlueprintSetLibrary.Set_ToArray` (`.Mappings` (break `KeyMappingRow` (`BlueprintMapLibrary.Map_Find` _returnvalue "MoveLeft")))))
                (bind _result_2 (`BlueprintSetLibrary.Set_ToArray` (`.Mappings` (break `KeyMappingRow` (`BlueprintMapLibrary.Map_Find` _returnvalue "MoveLeft_Secondary")))))
                (`InputMappingContext.UnmapAllKeysFromAction` _imc_notebookref_2 "/Game/MenuSystemPro/Blueprints/Input/CharacterOnFoot/IA_TurnPageLeft.IA_TurnPageLeft")
                (bind _returnvalue_2 (`InputMappingContext.MapKey` _imc_notebookref_2 "/Game/MenuSystemPro/Blueprints/Input/CharacterOnFoot/IA_TurnPageLeft.IA_TurnPageLeft" (`.CurrentKey` (break `PlayerKeyMapping` (`|GetArrayItem` _result)))))
                (bind _returnvalue_3 (`InputMappingContext.MapKey` _imc_notebookref_2 "/Game/MenuSystemPro/Blueprints/Input/CharacterOnFoot/IA_TurnPageLeft.IA_TurnPageLeft" (`.CurrentKey` (break `PlayerKeyMapping` (`|GetArrayItem` _result_2)))))
                (`KismetSystemLibrary.PrintText` (`KismetInputLibrary.Key_GetDisplayName` (`.Key` (break `EnhancedActionKeyMapping` _returnvalue_2))))
                (`KismetSystemLibrary.PrintText` (`KismetInputLibrary.Key_GetDisplayName` (`.Key` (break `EnhancedActionKeyMapping` _returnvalue_3)))))
              (:`then_1`
                (bind _result_3 (`BlueprintSetLibrary.Set_ToArray` (`.Mappings` (break `KeyMappingRow` (`BlueprintMapLibrary.Map_Find` _returnvalue "MoveRight_Secondary")))))
                (bind _result_4 (`BlueprintSetLibrary.Set_ToArray` (`.Mappings` (break `KeyMappingRow` (`BlueprintMapLibrary.Map_Find` _returnvalue "MoveRight")))))
                (`InputMappingContext.UnmapAllKeysFromAction` _imc_notebookref "/Game/MenuSystemPro/Blueprints/Input/CharacterOnFoot/IA_TurnPageRight.IA_TurnPageRight")
                (bind _returnvalue_4 (`InputMappingContext.MapKey` _imc_notebookref "/Game/MenuSystemPro/Blueprints/Input/CharacterOnFoot/IA_TurnPageRight.IA_TurnPageRight" (`.CurrentKey` (break `PlayerKeyMapping` (`|GetArrayItem` _result_4)))))
                (bind _returnvalue_5 (`InputMappingContext.MapKey` _imc_notebookref "/Game/MenuSystemPro/Blueprints/Input/CharacterOnFoot/IA_TurnPageRight.IA_TurnPageRight" (`.CurrentKey` (break `PlayerKeyMapping` (`|GetArrayItem` _result_3)))))
                (`KismetSystemLibrary.PrintText` (`KismetInputLibrary.Key_GetDisplayName` (`.Key` (break `EnhancedActionKeyMapping` _returnvalue_5))))
                (`KismetSystemLibrary.PrintText` (`KismetInputLibrary.Key_GetDisplayName` (`.Key` (break `EnhancedActionKeyMapping` _returnvalue_4))))
                (`EnhancedInputSubsystemInterface.AddMappingContext` (pcsubsystem `EnhancedInputLocalPlayerSubsystem` (`GameplayStatics.GetPlayerController` 0)) "/Game/MenuSystemPro/Blueprints/Input/CharacterOnFoot/IMC_Notebook.IMC_Notebook" 25 (struct))
                (`KismetSystemLibrary.PrintString` "Added")))))))
    (:`then_1`
      (`KismetSystemLibrary.Delay` 0.2))))

(event `Close`
  (set `self.Animation is Playing?` true)
  (set `self.AddMappingContext?` false)
  (`|ExecutionSequence`
    (:`then_0`
      (goto _label :!via `Reverse`))
    (:`then_1`
      (`KismetSystemLibrary.Delay` 0.2)
      (set `self.Book Opened?` false)
      (message `EnhancedInputSubsystemInterface.RemoveMappingContext` (pcsubsystem `EnhancedInputLocalPlayerSubsystem` (`GameplayStatics.GetPlayerController` 0)) "/Game/MenuSystemPro/Blueprints/Input/CharacterOnFoot/IMC_Notebook.IMC_Notebook" (make `ModifyContextOptions` true))
      (`KismetSystemLibrary.PrintString` "Removed"))))

(event `Try Turn Page Forward`
  (if (and (!= (+ (`self.Current Page`) 1) 61) (not (`self.Animation is Playing?`)))
    (bind _result (`/Engine/EditorBlueprintResources/StandardMacros.IncrementInt` (`self.Current Page`))
      (:`  `
        (`self.Turn Page Forward`)
        (`KismetSystemLibrary.PrintString` "fwd")
        (`KismetSystemLibrary.PrintString` (`KismetStringLibrary.Conv_IntToString` _result))))))

(event `Try Turn Page Backward`
  (if (and (!= (- (`self.Current Page`) 1) 0) (not (`self.Animation is Playing?`)))
    (bind _result (`/Engine/EditorBlueprintResources/StandardMacros.DecrementInt` (`self.Current Page`))
      (:`  `
        (`self.Turn Page Backward`)
        (`KismetSystemLibrary.PrintString` "bwd")
        (`KismetSystemLibrary.PrintString` (`KismetStringLibrary.Conv_IntToString` _result))))))

(event `Turn Page Forward`
  (bind _page_righttoleft (`self.Page RightToLeft`))
  (set `self.Animation is Playing?` true)
  (`SkeletalMeshComponent.SetPlayRate` _page_righttoleft 1.0)
  (`SkeletalMeshComponent.Play` _page_righttoleft false)
  (set `self.LeftPageDelayed?` false)
  (`self.Draw Page` (`self.Current Page`) :!label _label_2)
  (`KismetSystemLibrary.Delay` 2.0)
  (`SkeletalMeshComponent.SetPosition` (`self.Page LeftToRight`) 0.0 true)
  (`SkeletalMeshComponent.SetPosition` (`self.Page RightToLeft`) 0.0 true)
  (set `self.Animation is Playing?` false))

(event `Turn Page Backward`
  (bind _page_lefttoright (`self.Page LeftToRight`))
  (set `self.Animation is Playing?` true)
  (`SkeletalMeshComponent.SetPlayRate` _page_lefttoright 1.0)
  (`SkeletalMeshComponent.Play` _page_lefttoright false)
  (set `self.LeftPageDelayed?` true)
  (goto _label_2))

(event `Draw Page`
  (params (Index :type Integer))
  (`KismetSystemLibrary.Delay` 0.1)
  (switch `int` Index
    (:`1`
      (`self.Draw Page Helper` "/Game/Notebook/Pages/WB_NotebookPage1A.WB_NotebookPage1A_C" "/Game/Notebook/Pages/WB_NotebookPage1B.WB_NotebookPage1B_C"))
    (:`2`
      (`self.Draw Page Helper` "/Game/Notebook/Pages/WB_NotebookPage2A.WB_NotebookPage2A_C" "/Game/Notebook/Pages/WB_NotebookPage2B.WB_NotebookPage2B_C"))
    (:`3`
      (`self.Draw Page Helper` "/Game/Notebook/Pages/WB_NotebookPage3A.WB_NotebookPage3A_C" "/Game/Notebook/Pages/WB_NotebookPage3B.WB_NotebookPage3B_C"))
    (:`4`
      (`self.Draw Page Helper` "/Game/Notebook/Pages/WB_NotebookPage1A.WB_NotebookPage1A_C" "/Game/Notebook/Pages/WB_NotebookPage1B.WB_NotebookPage1B_C"))
    (:`5`
      (`self.Draw Page Helper` "/Game/Notebook/Pages/WB_NotebookPage2A.WB_NotebookPage2A_C" "/Game/Notebook/Pages/WB_NotebookPage2B.WB_NotebookPage2B_C"))))

(event `Draw Page Helper`
  (params (Left :type "UserWidget Class Reference") (Right :type "UserWidget Class Reference"))
  (bind _returnvalue (`|CreateWidget` Left))
  (bind _returnvalue_2 (`|CreateWidget` Right))
  (set `self.User Widget A` null)
  (set `self.User Widget B` null)
  (set `self.Prev User Widget A` null)
  (set `self.Prev user Widget B` null)
  (set `self.Prev User Widget A` (`WidgetComponent.GetWidget` (`self.Page A Widget`)))
  (set `self.Prev user Widget B` (`WidgetComponent.GetWidget` (`self.Page B  Widget`)))
  (set `self.User Widget A` _returnvalue)
  (set `self.User Widget B` _returnvalue_2)
  (if (`self.LeftPageDelayed?`)
    ;[1 1 1] Fix!
    (`|ExecutionSequence`
      (:`then_0`
        (`WidgetComponent.SetWidget` (`self.Page A Widget`) (`self.User Widget A`))
        (`KismetSystemLibrary.Delay` 1.1)
        (`WidgetComponent.SetWidget` (`self.Page B  Widget`) (`self.User Widget B`)))
      (:`then_1`
        (`WidgetComponent.SetWidget` (`self.Page B  Widget Copy`) (`self.Prev User Widget A`))
        (`WidgetComponent.SetWidget` (`self.Page A Widget Copy`) (`self.User Widget B`))))
    (else
      (`|ExecutionSequence`
        (:`then_0`
          (`WidgetComponent.SetWidget` (`self.Page B  Widget`) (`self.User Widget B`))
          (`KismetSystemLibrary.Delay` 1.1)
          (`WidgetComponent.SetWidget` (`self.Page A Widget`) (`self.User Widget A`)))
        (:`then_1`
          (`WidgetComponent.SetWidget` (`self.Page A Widget Copy`) (`self.User Widget A`))
          (`WidgetComponent.SetWidget` (`self.Page B  Widget Copy`) (`self.Prev user Widget B`)))))))

(fn `UserConstructionScript`)