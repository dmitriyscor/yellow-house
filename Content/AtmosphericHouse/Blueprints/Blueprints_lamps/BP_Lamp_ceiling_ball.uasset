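; Ceiling ball lamp Blueprint for the Atmospheric House, switched between lit and unlit looks by the LampOn flag.
; All logic runs in the Construction Script; the event graph holds only disabled stubs.
; When on, it applies the lit material to the base twice, leaving the ball untouched.
; When off, it destroys the point light, applies the unlit material to base and ball, and makes the ball Static.
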(fn `UserConstructionScript`
  (if (`self.Lamp On?`)
    (`PrimitiveComponent.SetMaterial` (`self.Lamp_ceiling_ball_base`) 0 "/Game/AtmosphericHouse/Materials/Clean/MI_Lamps_A_on_clean.MI_Lamps_A_on_clean")
    (`PrimitiveComponent.SetMaterial` (`self.Lamp_ceiling_ball_base`) 0 "/Game/AtmosphericHouse/Materials/Clean/MI_Lamps_A_on_clean.MI_Lamps_A_on_clean")
    (else
      (`ActorComponent.K2_DestroyComponent` (`self.PointLight`))
      (`PrimitiveComponent.SetMaterial` (`self.Lamp_ceiling_ball_base`) 0 "/Game/AtmosphericHouse/Materials/Clean/MI_Lamps_A_off_clean.MI_Lamps_A_off_clean")
      (`PrimitiveComponent.SetMaterial` (`self.Lamp_ceiling_ball_ball`) 0 "/Game/AtmosphericHouse/Materials/Clean/MI_Lamps_A_off_clean.MI_Lamps_A_off_clean")
      (`SceneComponent.SetMobility` (`self.Lamp_ceiling_ball_ball`) "Static"))))