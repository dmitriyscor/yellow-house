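; Master stairs building piece for the Atmospheric House set, assembled in the construction script.
; The Stairs selection and ExtraRailing flag pick which stair child actor component to add.
; For left or right variants, Floor and Ceiling toggles either raise that side's 6x3 pieces 300 units or destroy them, and the opposite side's pieces are removed.
; The basement variant removes all floor and ceiling pieces; the event graph is unused.
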(fn `UserConstructionScript`
  (bind _floor_6x3_stairs_l (`self.Floor_6x3_stairs_L`))
  (bind _ceiling_6x3_stairs_l (`self.Ceiling_6x3_stairs_L`))
  (bind _floor_6x3_stairs_l_2 (`self.Floor_6x3_stairs_L`))
  (bind _ceiling_6x3_stairs_l_2 (`self.Ceiling_6x3_stairs_L`))
  (bind _floor_6x3_stairs_r (`self.Floor_6x3_stairs_R`))
  (bind _ceiling_6x3_stairs_r (`self.Ceiling_6x3_stairs_R`))
  (bind _floor_6x3_stairs_r_2 (`self.Floor_6x3_stairs_R`))
  (bind _ceiling_6x3_stairs_r_2 (`self.Ceiling_6x3_stairs_R`))
  (if (`self.Extra Railing?`)
    (switch `/Game/AtmosphericHouse/Enums/E_Stairs` (`self.Stairs`)
      (:`NewEnumerator19`
        (`AddComponent|NODE_AddChildActorComponent-0`)
        (`ActorComponent.K2_DestroyComponent` (`self.Floor_6x3_stairs_L`) :!label _label)
        (`ActorComponent.K2_DestroyComponent` (`self.Ceiling_6x3_stairs_L`))
        (`ActorComponent.K2_DestroyComponent` (`self.Floor_6x3_stairs_R`) :!label _label_2)
        (`ActorComponent.K2_DestroyComponent` (`self.Ceiling_6x3_stairs_R`)))
      (:`NewEnumerator25`
        (`AddComponent|NODE_AddChildActorComponent-17`)
        (if (`self.Floor?`) :!label _label_3
          (`SceneComponent.K2_SetRelativeLocationAndRotation` :`self` _floor_6x3_stairs_l :`NewLocation` (0.0 0.0 300.0))
          (else
            (`ActorComponent.K2_DestroyComponent` _floor_6x3_stairs_l)))
        (if (`self.Ceiling?`)
          (`SceneComponent.K2_SetRelativeLocationAndRotation` :`self` _ceiling_6x3_stairs_l :`NewLocation` (0.0 0.0 300.0))
          (goto _label_2)
          (else
            (`ActorComponent.K2_DestroyComponent` _ceiling_6x3_stairs_l)
            (goto _label_2))))
      (:`NewEnumerator54`
        (`AddComponent|NODE_AddChildActorComponent-18`)
        (if (`self.Floor?`) :!label _label_4
          (`SceneComponent.K2_SetRelativeLocationAndRotation` :`self` _floor_6x3_stairs_r :`NewLocation` (0.0 0.0 300.0))
          (else
            (`ActorComponent.K2_DestroyComponent` _floor_6x3_stairs_r)))
        (if (`self.Ceiling?`)
          (`SceneComponent.K2_SetRelativeLocationAndRotation` :`self` _ceiling_6x3_stairs_r :`NewLocation` (0.0 0.0 300.0))
          (else
            (`ActorComponent.K2_DestroyComponent` _ceiling_6x3_stairs_r)))
        (`ActorComponent.K2_DestroyComponent` (`self.Floor_6x3_stairs_L`))
        (`ActorComponent.K2_DestroyComponent` (`self.Ceiling_6x3_stairs_L`)))
      (:`NewEnumerator55`
        (`AddComponent|NODE_AddChildActorComponent-19`)
        (goto _label_3))
      (:`NewEnumerator56`
        (`AddComponent|NODE_AddChildActorComponent-20`)
        (goto _label_4)))
    (else
      (switch `/Game/AtmosphericHouse/Enums/E_Stairs` (`self.Stairs`)
        (:`NewEnumerator19`
          (`AddComponent|NODE_AddChildActorComponent-21`)
          (goto _label))
        (:`NewEnumerator25`
          (`AddComponent|NODE_AddChildActorComponent-22`)
          (if (`self.Floor?`) :!label _label_5
            (`SceneComponent.K2_SetRelativeLocationAndRotation` :`self` _floor_6x3_stairs_l_2 :`NewLocation` (0.0 0.0 300.0))
            (else
              (`ActorComponent.K2_DestroyComponent` _floor_6x3_stairs_l_2)))
          (if (`self.Ceiling?`)
            (`SceneComponent.K2_SetRelativeLocationAndRotation` :`self` _ceiling_6x3_stairs_l_2 :`NewLocation` (0.0 0.0 300.0))
            (else
              (`ActorComponent.K2_DestroyComponent` _ceiling_6x3_stairs_l_2)))
          (`ActorComponent.K2_DestroyComponent` (`self.Floor_6x3_stairs_R`))
          (`ActorComponent.K2_DestroyComponent` (`self.Ceiling_6x3_stairs_R`)))
        (:`NewEnumerator54`
          (`AddComponent|NODE_AddChildActorComponent-23`)
          (if (`self.Floor?`) :!label _label_6
            (`SceneComponent.K2_SetRelativeLocationAndRotation` :`self` _floor_6x3_stairs_r_2 :`NewLocation` (0.0 0.0 300.0))
            (else
              (`ActorComponent.K2_DestroyComponent` _floor_6x3_stairs_r_2)))
          (if (`self.Ceiling?`)
            (`SceneComponent.K2_SetRelativeLocationAndRotation` :`self` _ceiling_6x3_stairs_r_2 :`NewLocation` (0.0 0.0 300.0))
            (else
              (`ActorComponent.K2_DestroyComponent` _ceiling_6x3_stairs_r_2)))
          (`ActorComponent.K2_DestroyComponent` (`self.Floor_6x3_stairs_L`))
          (`ActorComponent.K2_DestroyComponent` (`self.Ceiling_6x3_stairs_L`)))
        (:`NewEnumerator55`
          (`AddComponent|NODE_AddChildActorComponent-24`)
          (goto _label_5))
        (:`NewEnumerator56`
          (`AddComponent|NODE_AddChildActorComponent-25`)
          (goto _label_6))))))