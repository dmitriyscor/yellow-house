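; Configurable master door actor for the house building kit that assembles the selected door style at construction time.
; The Construction Script switches on the Doors choice and spawns child actor components for single A/B/C doors, mirrored double doors or a sliding pair.
; DoorRotation sets the swing angle, negated on the second leaf, while clamped SlidingDoorL and SlidingDoorR values set each sliding panel's offset.
; It has no runtime logic.
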(fn `UserConstructionScript`
  (bind _door_rotation (`self.Door Rotation`))
  (bind _returnvalue (`KismetMathLibrary.MakeTransform` (0.0 2.0 0.0) (`KismetMathLibrary.MakeRotator` 0.0 0.0 (`self.Door Rotation`))))
  (bind _returnvalue_2 (`KismetMathLibrary.MakeTransform` (0.0 -98.449997 0.0) (`KismetMathLibrary.MakeRotator` 0.0 0.0 _door_rotation)))
  (bind _returnvalue_3 (`KismetMathLibrary.MakeTransform` (0.0 98.449997 0.0) (`KismetMathLibrary.MakeRotator` 0.0 0.0 (* _door_rotation -1.0))))
  (switch `/Game/AtmosphericHouse/Enums/E_Doors` (`self.Doors`)
    (:`NewEnumerator19`
      (`AddComponent|NODE_AddChildActorComponent-0` :`RelativeTransform` _returnvalue))
    (:`NewEnumerator43`
      (`AddComponent|NODE_AddChildActorComponent-4` :`RelativeTransform` _returnvalue))
    (:`NewEnumerator45`
      (`AddComponent|NODE_AddChildActorComponent-7` :`RelativeTransform` _returnvalue))
    (:`NewEnumerator47`
      (`AddComponent|NODE_AddChildActorComponent-9` :`RelativeTransform` _returnvalue_2)
      (`AddComponent|NODE_AddChildActorComponent-10` :`RelativeTransform` _returnvalue_3))
    (:`NewEnumerator48`
      (`AddComponent|NODE_AddChildActorComponent-11` :`RelativeTransform` _returnvalue_2)
      (`AddComponent|NODE_AddChildActorComponent-12` :`RelativeTransform` _returnvalue_3))
    (:`NewEnumerator49`
      (`AddComponent|NODE_AddChildActorComponent-13` :`RelativeTransform` _returnvalue_2)
      (`AddComponent|NODE_AddChildActorComponent-14` :`RelativeTransform` _returnvalue_3))
    (:`NewEnumerator50`
      (`AddComponent|NODE_AddChildActorComponent-15` :`RelativeTransform` (`KismetMathLibrary.MakeTransform` (`KismetMathLibrary.MakeVector` 0.0 (`KismetMathLibrary.MapRangeClamped` (`self.Sliding Door L`) 0.0 1.0 1.0 99.0))))
      (`AddComponent|NODE_AddChildActorComponent-16` :`RelativeTransform` (`KismetMathLibrary.MakeTransform` (`KismetMathLibrary.MakeVector` 0.0 (* (`KismetMathLibrary.MapRangeClamped` (`self.Sliding Door R`) 0.0 1.0 1.0 99.0) -1.0)) (struct :`Yaw` 180.0))))))