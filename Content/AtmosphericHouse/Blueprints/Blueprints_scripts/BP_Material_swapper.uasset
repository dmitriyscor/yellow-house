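; Editor utility actor that swaps materials on static mesh components across every actor in the level from its construction script.
; Setting UpdateMaterials triggers one pass, which then resets the flag.
; It either flips all materials between clean and worn sets by substituting _clean/_worn name suffixes, or replaces one named material with another from both lists.
; Wildcard name matching runs in deeply nested loops, so the project's Max Loop Count must be raised.
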(fn `UserConstructionScript`
  (if (`self.Update Materials`)
    ;[1 1 1] Set Max Loop Count to 2 000 000 from Project Settings
    (if (`self.Swap Individual Materials`)
      (`KismetArrayLibrary.Array_Clear` (`self.Materials_all`))
      (`KismetArrayLibrary.Array_Append` (`self.Materials_all`) (`self.Materials_clean`))
      (`KismetArrayLibrary.Array_Append` (`self.Materials_all`) (`self.Materials_worn`))
      (bind _outactors (`GameplayStatics.GetAllActorsOfClass` "/Script/Engine.Actor"))
      (for _array_element _outactors
        (for _array_element_2 (`self.K2_GetComponentsByClass` _array_element "/Script/Engine.StaticMeshComponent")
          (for (_array_element_3 _array_index) (`MeshComponent.GetMaterials` _array_element_2)
            (if (`KismetStringLibrary.MatchesWildcard` (`KismetStringLibrary.Conv_ObjectToString` _array_element_3) (`self.Current Material Name`))
              (for _array_element_4 (`self.Materials_all`)
                (if (`KismetStringLibrary.MatchesWildcard` (`self.New Assigned  Material Name`) (`KismetStringLibrary.Conv_ObjectToString` _array_element_4))
                  (`PrimitiveComponent.SetMaterial` _array_element_2 _array_index _array_element_4)))))))
      (set `self.Update Materials` false)
      (elif (`self.Worn Materials`)
        (bind _outactors_2 (`GameplayStatics.GetAllActorsOfClass` "/Script/Engine.Actor"))
        (for _array_element_5 _outactors_2
          (for _array_element_6 (`self.K2_GetComponentsByClass` _array_element_5 "/Script/Engine.StaticMeshComponent")
            (for (_array_element_7 _array_index_2) (`MeshComponent.GetMaterials` _array_element_6)
              (for _array_element_8 (`self.Materials_worn`)
                (if (`KismetStringLibrary.MatchesWildcard` (`KismetStringLibrary.Replace` (`KismetStringLibrary.Conv_ObjectToString` _array_element_7) "_clean" "_worn") (`KismetStringLibrary.Conv_ObjectToString` _array_element_8))
                  (`PrimitiveComponent.SetMaterial` _array_element_6 _array_index_2 _array_element_8))))))
        (set `self.Update Materials` false)
        (else
          (bind _outactors_3 (`GameplayStatics.GetAllActorsOfClass` "/Script/Engine.Actor"))
          (for _array_element_9 _outactors_3
            (for _array_element_10 (`self.K2_GetComponentsByClass` _array_element_9 "/Script/Engine.StaticMeshComponent")
              (for (_array_element_11 _array_index_3) (`MeshComponent.GetMaterials` _array_element_10)
                (for _array_element_12 (`self.Materials_clean`)
                  (if (`KismetStringLibrary.MatchesWildcard` (`KismetStringLibrary.Replace` (`KismetStringLibrary.Conv_ObjectToString` _array_element_11) "_worn" "_clean") (`KismetStringLibrary.Conv_ObjectToString` _array_element_12))
                    (`PrimitiveComponent.SetMaterial` _array_element_10 _array_index_3 _array_element_12))))))
          (set `self.Update Materials` false))))))