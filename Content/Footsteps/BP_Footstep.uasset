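; Animation notify that plays surface-specific footstep sounds for the animated mesh's owner.
; When fired, it traces 200 units down from the owner's location on the Visibility channel and reads the hit's physical surface type.
; PlaySound switches on that surface to play a matching cue at the owner's location, not at the foot.
; Surfaces without a case, including the default, play no sound.
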(fn `PlaySound`
  (params (`E Physical Surface Enum` :type "EPhysicalSurface Enum" :default "SurfaceType_Default") (Location :type "Vector Structure"))
  (bind _location (`local.Location`))
  (bind _location_2 (`local.Location`))
  (bind _location_3 (`local.Location`))
  (bind _location_4 (`local.Location`))
  (bind _location_5 (`local.Location`))
  (bind _location_6 (`local.Location`))
  (switch `EPhysicalSurface` `E Physical Surface Enum`
    (:`SurfaceType1`
      (`GameplayStatics.PlaySoundAtLocation` "/Game/Footsteps/SoundCue/DIrtRoad_Cue.DIrtRoad_Cue" _location (struct) 1.0 1.0 0.0 "/Game/Footsteps/ATT_Footsteps.ATT_Footsteps" null null null))
    (:`SurfaceType2`
      (`GameplayStatics.PlaySoundAtLocation` "/Game/Footsteps/SoundCue/Glass_Cue.Glass_Cue" _location (struct) 1.0 1.0 0.0 "/Game/Footsteps/ATT_Footsteps.ATT_Footsteps" null null null))
    (:`SurfaceType3`
      (`GameplayStatics.PlaySoundAtLocation` "/Game/Footsteps/SoundCue/Ice_Cue.Ice_Cue" _location (struct) 1.0 1.0 0.0 "/Game/Footsteps/ATT_Footsteps.ATT_Footsteps" null null null))
    (:`SurfaceType4`
      (`GameplayStatics.PlaySoundAtLocation` "/Game/Footsteps/SoundCue/Linoleum_Cue.Linoleum_Cue" _location_6 (struct) 1.0 1.0 0.0 "/Game/Footsteps/ATT_Footsteps.ATT_Footsteps" null null null))
    (:`SurfaceType5`
      (`GameplayStatics.PlaySoundAtLocation` "/Game/Footsteps/SoundCue/LowMetal_Cue.LowMetal_Cue" _location_6 (struct) 1.0 1.0 0.0 "/Game/Footsteps/ATT_Footsteps.ATT_Footsteps" null null null))
    (:`SurfaceType6`
      (`GameplayStatics.PlaySoundAtLocation` "/Game/Footsteps/SoundCue/Metal_Cue.Metal_Cue" _location_5 (struct) 1.0 1.0 0.0 "/Game/Footsteps/ATT_Footsteps.ATT_Footsteps" null null null))
    (:`SurfaceType7`
      (`GameplayStatics.PlaySoundAtLocation` "/Game/Footsteps/SoundCue/Mud_Cue.Mud_Cue" _location_5 (struct) 1.0 1.0 0.0 "/Game/Footsteps/ATT_Footsteps.ATT_Footsteps" null null null))
    (:`SurfaceType8`
      (`GameplayStatics.PlaySoundAtLocation` "/Game/Footsteps/SoundCue/Parquete_Cue.Parquete_Cue" _location_4 (struct) 1.0 1.0 0.0 "/Game/Footsteps/ATT_Footsteps.ATT_Footsteps" null null null))
    (:`SurfaceType9`
      (`GameplayStatics.PlaySoundAtLocation` "/Game/Footsteps/SoundCue/PavementTilse_Cue.PavementTilse_Cue" _location_4 (struct) 1.0 1.0 0.0 "/Game/Footsteps/ATT_Footsteps.ATT_Footsteps" null null null))
    (:`SurfaceType10`
      (`GameplayStatics.PlaySoundAtLocation` "/Game/Footsteps/SoundCue/Snow_Cue.Snow_Cue" _location_3 (struct) 1.0 1.0 0.0 "/Game/Footsteps/ATT_Footsteps.ATT_Footsteps" null null null))
    (:`SurfaceType11`
      (`GameplayStatics.PlaySoundAtLocation` "/Game/Footsteps/SoundCue/TallGrass_Cue.TallGrass_Cue" _location_3 (struct) 1.0 1.0 0.0 "/Game/Footsteps/ATT_Footsteps.ATT_Footsteps" null null null))
    (:`SurfaceType12`
      (`GameplayStatics.PlaySoundAtLocation` "/Game/Footsteps/SoundCue/Tiles_Cue.Tiles_Cue" _location_2 (struct) 1.0 1.0 0.0 "/Game/Footsteps/ATT_Footsteps.ATT_Footsteps" null null null))
    (:`SurfaceType13`
      (`GameplayStatics.PlaySoundAtLocation` "/Game/Footsteps/SoundCue/Undergrows_Cue.Undergrows_Cue" _location_2 (struct) 1.0 1.0 0.0 "/Game/Footsteps/ATT_Footsteps.ATT_Footsteps" null null null))))

(fn `Received_Notify`
  (params (MeshComp :type "SkeletalMeshComponent Object Reference") (Animation :type "AnimSequenceBase Object Reference") (EventReference :type "AnimNotifyEventReference Structure (by ref)"))
  (returns (ReturnValue :type Boolean))
  (bind _returnvalue (`ActorComponent.GetOwner` MeshComp))
  (bind _returnvalue_2 (`Actor.K2_GetActorLocation` _returnvalue))
  (bind (_outhit _returnvalue_3) (`KismetSystemLibrary.LineTraceSingle` _returnvalue_2 (+ _returnvalue_2 (* (`Actor.GetActorUpVector` _returnvalue) -200)) "TraceTypeQuery1"))
  (if _returnvalue_3
    (`self.PlaySound` (`GameplayStatics.GetSurfaceType` _outhit) _returnvalue_2)
    (return true)))