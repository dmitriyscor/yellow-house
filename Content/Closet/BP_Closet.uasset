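; BP_Closet is a closet whose two doors swing open and shut when a monster checks it.
; Playanim and PlayMonsterChecksClosetAnimation share one sequence: the MonsterCheck timeline opens both doors, then ClosetCloses shuts them after a pause, held longer if PlayerInside is set.
; AnimationPlaying only delays an overlapping call briefly rather than blocking it.
; Player enter and exit animation events are empty stubs.
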(event `Play Player Enter Animation`
  ;[1 1 1] Player
)

(event `Play anim`
  ;[1 1 1] Monster
  (if (`self.Animation Playing?`) :!label _label
    (`KismetSystemLibrary.Delay` 0.5))
  (set `self.Animation Playing?` true)
  (bind (_direction _open) (`Timeline|Monster Check` :!via `PlayFromStart`)
    (:`Update`
      (`SceneComponent.K2_SetRelativeRotation` (`self.02_3_02_0`) (`KismetMathLibrary.MakeRotator` 0.0 0.0 (`KismetMathLibrary.Lerp` 0.0 160.0 _open)) false false)
      (`SceneComponent.K2_SetRelativeRotation` (`self.02_2_02_0`) (`KismetMathLibrary.MakeRotator` 0.0 0.0 (`KismetMathLibrary.Lerp` 0.0 -160.0 _open)) false false))
    (:`Finished`
      (`KismetSystemLibrary.Delay` 2.0)
      (if (`self.Player Inside?`)
        (`KismetSystemLibrary.Delay` 3.0)
        (bind (_direction_2 _open_2) (`Timeline|Closet Closes` :!via `PlayFromStart` :!label _label_2)
          (:`Update`
            (`SceneComponent.K2_SetRelativeRotation` (`self.02_3_02_0`) (`KismetMathLibrary.MakeRotator` 0.0 0.0 (`KismetMathLibrary.Lerp` 160.0 0.0 _open_2)) false false)
            (`SceneComponent.K2_SetRelativeRotation` (`self.02_2_02_0`) (`KismetMathLibrary.MakeRotator` 0.0 0.0 (`KismetMathLibrary.Lerp` -160.0 0.0 _open_2)) false false))
          (:`Finished`
            (set `self.Animation Playing?` false)))
        (else
          (goto _label_2 :!via `PlayFromStart`))))))

(event `Play Monster Checks Closet Animation`
  ;[1 1 1] Monster
  (goto _label))

(event `Play Player Exit Animation`
  ;[1 1 1] Player
)

(fn `UserConstructionScript`)