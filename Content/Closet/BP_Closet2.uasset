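; BP_Closet2 is a closet Blueprint that animates a sliding part, likely the door, when the monster checks the closet.
; Playanim and PlayMonsterChecksClosetAnimation share one sequence: a timeline lerps the object's relative Y open, and a second timeline closes it after a pause.
; The pause is longer when PlayerInside is set, and AnimationPlaying tracks the running sequence.
; Interact tests both flags but performs no action.
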(event `Play anim`
  (bind _object (`self.Object`))
  (bind _object_2 (`self.Object`))
  (bind (_relativelocation_x _relativelocation_y _relativelocation_z) (`KismetMathLibrary.BreakVector` (`SceneComponent.RelativeLocation` _object)))
  (bind (_relativelocation_x_2 _relativelocation_y_2 _relativelocation_z_2) (`KismetMathLibrary.BreakVector` (`SceneComponent.RelativeLocation` _object_2)))
  ;[1 1 1] Monster
  (if (`self.Animation Playing?`) :!label _label
    (`KismetSystemLibrary.Delay` 0.5))
  (set `self.Animation Playing?` true)
  (bind (_direction _open) (`Timeline|Timeline` :!via `PlayFromStart`)
    (:`Update`
      (`SceneComponent.K2_SetRelativeLocation` _object_2 (`KismetMathLibrary.MakeVector` _relativelocation_x_2 (`KismetMathLibrary.Lerp` -3.0 -65.0 _open) _relativelocation_z_2) false false))
    (:`Finished`
      (`KismetSystemLibrary.Delay` 2.0)
      (if (`self.Player Inside?`)
        (`KismetSystemLibrary.Delay` 3.0)
        (bind (_direction_2 _open_2) (`Timeline|Timeline_0` :!via `PlayFromStart` :!label _label_2)
          (:`Update`
            (`SceneComponent.K2_SetRelativeLocation` _object (`KismetMathLibrary.MakeVector` _relativelocation_x (`KismetMathLibrary.Lerp` -65.0 -3.0 _open_2) _relativelocation_z) false false))
          (:`Finished`
            (set `self.Animation Playing?` false)))
        (else
          (goto _label_2 :!via `PlayFromStart`))))))

(event `Play Monster Checks Closet Animation`
  ;[1 1 1] Monster
  (goto _label))

(event `/Game/ThirdPerson/Blueprints/BPI_Interaction.Interact`
  (if (`self.Animation Playing?`)
    (if (`self.Player Inside?`)
      _)))

(fn `UserConstructionScript`
  (`parent.UserConstructionScript`))