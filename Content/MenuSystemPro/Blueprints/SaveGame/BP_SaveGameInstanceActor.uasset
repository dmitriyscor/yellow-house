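; One-off actor, spawned by BP_SaveGameManager, that saves, loads or initializes a BP_CustomSaveGameObject with world access, as overridable functions.
; Saving records level, play time, timestamp, save count, player transform and random placeholder mission text, then writes the slot.
; Loading restores play time through BPI_GameInstanceExtension and opens the saved level; it does not apply the saved transform.
; New games start with fresh metadata.
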(fn `CreateNewSaveGame`
  (params (AreaName :type Name) (SaveGame :type "SaveGame Object Reference") (SlotName :type String))
  ;[1 1 1] Used when creating a new game. Override this function to use your own SaveGame object
  (bind _asbp_custom_save_game_object (cast `/Game/MenuSystemPro/Blueprints/SaveGame/BP_CustomSaveGameObject` SaveGame))
  (set `/Game/MenuSystemPro/Blueprints/SaveGame/BP_CustomSaveGameObject.AreaName` AreaName _asbp_custom_save_game_object)
  (set `/Game/MenuSystemPro/Blueprints/SaveGame/BP_CustomSaveGameObject.LastSavedTimestamp` (`KismetMathLibrary.Now`) _asbp_custom_save_game_object)
  (set `/Game/MenuSystemPro/Blueprints/SaveGame/BP_CustomSaveGameObject.SavesCount` 1 _asbp_custom_save_game_object)
  (set `/Game/MenuSystemPro/Blueprints/SaveGame/BP_CustomSaveGameObject.PlayTimeInSeconds` 0.0 _asbp_custom_save_game_object)
  (set `/Game/MenuSystemPro/Blueprints/SaveGame/BP_CustomSaveGameObject.AreaText` (select `int` (`KismetMathLibrary.RandomIntegerInRange` 0 3) :`0` "Find a way out" :`1` "Escape the town" :`2` "Find Basement Key" :`3` "Find the hiden door" :!type "Name") _asbp_custom_save_game_object) ; Set this dynamically with your game logic \n(e.g. run into a trigger changes this or saving at a certain location)
)

(fn `LoadGame`
  (params (SlotName :type String) (UserIndex :type Integer))
  (returns (SaveGame :type "SaveGame Object Reference"))
  ;[1 1 1] Load Game - Consider that anything you apply to your current level is lost when you travel to the next level.
  ; Changes to your Player Character and other Actors in your loaded level need to be made AFTER the level has opened.
  ; This can for example be the 'Begin Play' event of an actor. You can access the loaded SaveGameObject via GameInstance -> BP_SaveGameManager
  (bind _returnvalue (`GameplayStatics.LoadGameFromSlot` SlotName UserIndex))
  (bind _asbp_custom_save_game_object (cast `/Game/MenuSystemPro/Blueprints/SaveGame/BP_CustomSaveGameObject` _returnvalue))
  (bind _asbpi_game_instance_extension (cast `/Game/MenuSystemPro/Blueprints/GameFramework/BPI_GameInstanceExtension` (`GameplayStatics.GetGameInstance`)))
  (`/Game/MenuSystemPro/Blueprints/GameFramework/BPI_GameInstanceExtension.OnSetCurrentPlayTime` _asbpi_game_instance_extension (`/Game/MenuSystemPro/Blueprints/SaveGame/BP_CustomSaveGameObject.PlayTimeInSeconds` _asbp_custom_save_game_object))
  ;[1 1 1] Open Level
  (`/Game/MenuSystemPro/Blueprints/GameFramework/BPI_GameInstanceExtension.OnOpenLevel` _asbpi_game_instance_extension (`/Game/MenuSystemPro/Blueprints/SaveGame/BP_CustomSaveGameObject.AreaName` _asbp_custom_save_game_object) true "")
  (return _returnvalue))

(fn `SaveGame`
  (params (SaveGameObject :type "SaveGame Object Reference") (SlotName :type String) (UserIndex :type Integer))
  (returns (bSuccess :type Boolean))
  ;[1 1 1] Set Custom Save Game Object Data while saving. Override this function to use your own SaveGame object
  (`|ExecutionSequence`
    (:`then_0`
      (bind _asbp_custom_save_game_object (cast `/Game/MenuSystemPro/Blueprints/SaveGame/BP_CustomSaveGameObject` SaveGameObject))
      (bind _asbpi_game_instance_extension (cast `/Game/MenuSystemPro/Blueprints/GameFramework/BPI_GameInstanceExtension` (`GameplayStatics.GetGameInstance`)))
      (bind _currentlevelname (`/Game/MenuSystemPro/Blueprints/GameFramework/BPI_GameInstanceExtension.GetCurrentLevel` _asbpi_game_instance_extension))
      (set `/Game/MenuSystemPro/Blueprints/SaveGame/BP_CustomSaveGameObject.AreaName` _currentlevelname _asbp_custom_save_game_object)
      (set `/Game/MenuSystemPro/Blueprints/SaveGame/BP_CustomSaveGameObject.AreaText` (select `int` (`KismetMathLibrary.RandomIntegerInRange` 0 3) :`0` "Find a way out" :`1` "Escape the town" :`2` "Find Basement Key" :`3` "Find the hiden door" :!type "Name") _asbp_custom_save_game_object) ; Set this dynamically with your game logic \n(e.g. run into a trigger changes this or saving at a certain location)
      (set `/Game/MenuSystemPro/Blueprints/SaveGame/BP_CustomSaveGameObject.SavesCount` (+ (`/Game/MenuSystemPro/Blueprints/SaveGame/BP_CustomSaveGameObject.SavesCount` _asbp_custom_save_game_object) 1) _asbp_custom_save_game_object)
      (bind _playtimeinseconds (`/Game/MenuSystemPro/Blueprints/GameFramework/BPI_GameInstanceExtension.GetCurrentPlayTime` _asbpi_game_instance_extension))
      (bind _output_get (set `/Game/MenuSystemPro/Blueprints/SaveGame/BP_CustomSaveGameObject.PlayTimeInSeconds` _playtimeinseconds _asbp_custom_save_game_object))
      (`/Game/MenuSystemPro/Blueprints/GameFramework/BPI_GameInstanceExtension.OnSetCurrentPlayTime` _asbpi_game_instance_extension _output_get)
      (set `/Game/MenuSystemPro/Blueprints/SaveGame/BP_CustomSaveGameObject.LastSavedTimestamp` (`KismetMathLibrary.Now`) _asbp_custom_save_game_object)
      (set `/Game/MenuSystemPro/Blueprints/SaveGame/BP_CustomSaveGameObject.PlayerTransform` (`self.GetTransform` (`GameplayStatics.GetPlayerCharacter` 0)) _asbp_custom_save_game_object))
    (:`then_1`
      ;[1 1 1] Save Game to Slot
      (bind _returnvalue (`GameplayStatics.SaveGameToSlot` SaveGameObject SlotName UserIndex))
      (return _returnvalue))))

(fn `UserConstructionScript`)