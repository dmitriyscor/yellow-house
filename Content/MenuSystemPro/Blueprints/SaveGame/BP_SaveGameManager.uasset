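; Save game manager for the menu system that creates, loads and saves slot-based games, held in a BP_CustomSaveGameObject.
; It is a UObject that uses its outer's BPI_GameInstanceExtension to spawn a temporary BP_SaveGameInstanceActor, which does the work and is then destroyed.
; Creating a game overwrites the slot, then loads it.
; Numbered-slot scans detect existing saves and find the newest by timestamp for Continue, reading metadata without opening levels.
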(fn `AnySaveGameExists`
  (params (SlotPrefix :type String :default "savegame_") (Amount :type Integer :default 20) (UserIndex :type Integer))
  (returns (bSaveGameExists :type Boolean))
  ;[1 1 1] Returns true if any savegame exists in Project/Saved/ folder with the matching slot name
  (for _index (range 1 (+ Amount 1))
    (bind _returnvalue (`GameplayStatics.DoesSaveGameExist` (`KismetStringLibrary.Concat_StrStr` SlotPrefix (`KismetStringLibrary.Conv_IntToString` _index)) UserIndex))
    (if _returnvalue
      (return true)))
  (return false))

(fn `CreateNewGame`
  (params (SlotName :type String) (UserIndex :type Integer) (LevelName :type Name))
  (returns (bSuccess :type Boolean))
  ;[1 1 1] Create New Game
  (bind _returnvalue (`GameplayStatics.DoesSaveGameExist` SlotName UserIndex))
  (if _returnvalue
    (`GameplayStatics.DeleteGameInSlot` SlotName UserIndex))
  (`self.CreateNewSaveGameObject` LevelName SlotName)
  (bind _returnvalue_2 (`GameplayStatics.SaveGameToSlot` (`self.SaveGameObject`) SlotName UserIndex))
  (`self.LoadGame` SlotName UserIndex)
  (return _returnvalue_2))

(fn `CreateNewSaveGameObject`
  (params (AreaName :type Name) (SlotName :type String))
  ;[1 1 1] Used when creating a new game.
  (bind _asbpi_game_instance_extension (cast `/Game/MenuSystemPro/Blueprints/GameFramework/BPI_GameInstanceExtension` (`KismetSystemLibrary.GetOuterObject` self)))
  (bind _actor (`/Game/MenuSystemPro/Blueprints/GameFramework/BPI_GameInstanceExtension.SpawnActor` :`self` _asbpi_game_instance_extension :`Class` "/Game/MenuSystemPro/Blueprints/SaveGame/BP_SaveGameInstanceActor.BP_SaveGameInstanceActor_C" :`CollisionHandlingOverride` "AlwaysSpawn"))
  (bind _asbp_save_game_instance_actor (cast `/Game/MenuSystemPro/Blueprints/SaveGame/BP_SaveGameInstanceActor` _actor))
  (`/Game/MenuSystemPro/Blueprints/SaveGame/BP_SaveGameInstanceActor.CreateNewSaveGame` _asbp_save_game_instance_actor AreaName (`self.SaveGameObject`) (`local.SlotName`))
  (`Actor.K2_DestroyActor` _asbp_save_game_instance_actor))

(fn `GetLatestSaveGame`
  (params (SlotPrefix :type String :default "savegame_") (UserIndex :type Integer) (Amount :type Integer :default 20))
  (returns (Success :type Boolean) (SlotName :type String))
  (locals (LatestSaveTimestamp :type "DateTime Structure") (LatestSaveSlot :type String))
  ;[1 1 1] Loads the most recent savegame. Used by the 'Continue' button in the Singleplayer Menu
  (for _index (range 1 (+ Amount 1))
    (bind _returnvalue (`KismetStringLibrary.Concat_StrStr` SlotPrefix (`KismetStringLibrary.Conv_IntToString` _index)))
    (bind _returnvalue_2 (`GameplayStatics.DoesSaveGameExist` _returnvalue UserIndex))
    (if _returnvalue_2
      (bind _savegameobject (`self.LoadSaveMetaData` _returnvalue))
      (bind _asbp_custom_save_game_object (cast `/Game/MenuSystemPro/Blueprints/SaveGame/BP_CustomSaveGameObject` _savegameobject))
      (bind _lastsavedtimestamp (`/Game/MenuSystemPro/Blueprints/SaveGame/BP_CustomSaveGameObject.LastSavedTimestamp` _asbp_custom_save_game_object))
      (if (> _lastsavedtimestamp (`local.LatestSaveTimestamp`))
        (set `local.LatestSaveTimestamp` _lastsavedtimestamp)
        (set `local.LatestSaveSlot` _returnvalue))))
  (return (not (`KismetStringLibrary.IsEmpty` (`local.LatestSaveSlot`))) (`local.LatestSaveSlot`)))

(fn `Initialize`
  ;[1 1 1] Init
  (cast `/Game/MenuSystemPro/Blueprints/GameFramework/BPI_GameInstanceExtension` (`KismetSystemLibrary.GetOuterObject` self))
  (bind _returnvalue (`GameplayStatics.CreateSaveGameObject` "/Game/MenuSystemPro/Blueprints/SaveGame/BP_CustomSaveGameObject.BP_CustomSaveGameObject_C"))
  (set `self.SaveGameObject` _returnvalue)
  (return))

(fn `LoadGame`
  (params (SlotName :type String) (UserIndex :type Integer))
  (returns (SaveGameObject :type "SaveGame Object Reference"))
  ;[1 1 1] Load from hard drive
  (bind _output_get (set `self.LastLoadedSaveSlotName` SlotName))
  (bind _asbpi_game_instance_extension (cast `/Game/MenuSystemPro/Blueprints/GameFramework/BPI_GameInstanceExtension` (`KismetSystemLibrary.GetOuterObject` self)))
  (bind _actor (`/Game/MenuSystemPro/Blueprints/GameFramework/BPI_GameInstanceExtension.SpawnActor` :`self` _asbpi_game_instance_extension :`Class` "/Game/MenuSystemPro/Blueprints/SaveGame/BP_SaveGameInstanceActor.BP_SaveGameInstanceActor_C" :`CollisionHandlingOverride` "AlwaysSpawn"))
  (bind _asbp_save_game_instance_actor (cast `/Game/MenuSystemPro/Blueprints/SaveGame/BP_SaveGameInstanceActor` _actor))
  (bind _savegame (`/Game/MenuSystemPro/Blueprints/SaveGame/BP_SaveGameInstanceActor.LoadGame` _asbp_save_game_instance_actor _output_get UserIndex))
  (set `self.SaveGameObject` _savegame)
  (`Actor.K2_DestroyActor` _asbp_save_game_instance_actor)
  (return (`self.SaveGameObject`)))

(fn `LoadSaveMetaData`
  (params (SlotName :type String) (UserIndex :type Integer))
  (returns (SaveGameObject :type "SaveGame Object Reference"))
  ;[1 1 1] Load without opening the level, this allows to e.g. setup the Save Game Slots in the Menu
  (bind _returnvalue (`GameplayStatics.LoadGameFromSlot` SlotName UserIndex))
  (return _returnvalue))

(fn `SaveGame`
  (params (SlotName :type String) (UserIndex :type Integer))
  (returns (bSuccess :type Boolean))
  ;[1 1 1] Save Game to hard drive
  (bind _asbpi_game_instance_extension (cast `/Game/MenuSystemPro/Blueprints/GameFramework/BPI_GameInstanceExtension` (`KismetSystemLibrary.GetOuterObject` self)))
  (bind _actor (`/Game/MenuSystemPro/Blueprints/GameFramework/BPI_GameInstanceExtension.SpawnActor` :`self` _asbpi_game_instance_extension :`Class` "/Game/MenuSystemPro/Blueprints/SaveGame/BP_SaveGameInstanceActor.BP_SaveGameInstanceActor_C" :`CollisionHandlingOverride` "AlwaysSpawn"))
  (bind _asbp_save_game_instance_actor (cast `/Game/MenuSystemPro/Blueprints/SaveGame/BP_SaveGameInstanceActor` _actor))
  (bind _bsuccess (`/Game/MenuSystemPro/Blueprints/SaveGame/BP_SaveGameInstanceActor.SaveGame` _asbp_save_game_instance_actor (`self.SaveGameObject`) (`local.SlotName`) (`local.UserIndex`)))
  (`Actor.K2_DestroyActor` _asbp_save_game_instance_actor)
  (return _bsuccess))