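; Trigger actor that autosaves the game when a player-controlled Character begins overlapping it.
; It gets the save game manager from the GameInstance through BPI_GameInstanceExtension and saves to the last loaded slot name.
; If no slot was loaded earlier, it skips saving and prints a warning; a successful save also prints the slot name.
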(event `self.ReceiveActorBeginOverlap`
  (params (OtherActor :type "Actor Object Reference"))
  ;[1 1 1] Check if character is player controlled
  (bind _ascharacter (cast `Character` OtherActor))
  (cast `PlayerController` (`Pawn.GetController` _ascharacter))
  ;[1 1 1] Save to last loaded save slot
  (bind _asbpi_game_instance_extension (cast `/Game/MenuSystemPro/Blueprints/GameFramework/BPI_GameInstanceExtension` (`GameplayStatics.GetGameInstance`)))
  (bind _savegamemanager (`/Game/MenuSystemPro/Blueprints/GameFramework/BPI_GameInstanceExtension.GetSaveGameManager` _asbpi_game_instance_extension))
  (bind _output (`|ConvertAsset` _savegamemanager))
  (bind _lastloadedsaveslotname (`/Game/MenuSystemPro/Blueprints/SaveGame/BP_SaveGameManager.LastLoadedSaveSlotName` _output))
  (if (not (`KismetStringLibrary.IsEmpty` _lastloadedsaveslotname))
    (`/Game/MenuSystemPro/Blueprints/SaveGame/BP_SaveGameManager.SaveGame` _output _lastloadedsaveslotname 0)
    (`KismetSystemLibrary.PrintString` (`KismetStringLibrary.Concat_StrStr` "Auto Save Trigger - Saved to Slot " _lastloadedsaveslotname))
    (else
      (`KismetSystemLibrary.PrintString` "Auto Save Trigger - No Valid Last Save Slot found. Make sure to test this by loading a game beforehand!"))))

(fn `UserConstructionScript`)